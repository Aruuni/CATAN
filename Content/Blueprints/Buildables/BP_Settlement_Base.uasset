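; Clickable settlement building for a Catan-style board game that the player can buy, upgrade to a city or steal from.
; On click it asks GameManager for the current player and only acts on PLAYER1's turn.
; An owned settlement attempts an upgrade; otherwise it tries stealing a resource, then buying if BoughtChecker returns false.
; Outcomes are mostly reported through Notification_HUD popups, with game rules delegated to functions defined outside this graph.
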(event MouseInput|EventActorOnClicked
  (params (ButtonPressed :type Key%20Structure :default "None"))
  (bind _returnvalue (Actor|GetActorOfClass "/Script/The_Settlers.GameManager"))
  (bind _returnvalue_2 (Class|GameManager|GetCurrentPlayer _returnvalue))
  (if (Utilities|Enum|Equal(Enum) _returnvalue_2 "PLAYER1")
    (bind _returnvalue_3 (Class|Settlement|GetOwner))
    (if (Utilities|Enum|Equal(Enum) _returnvalue_3 "PLAYER1")
      (bind _returnvalue_4 (Class|Settlement|Upgrade "PLAYER1"))
      (if _returnvalue_4
        (bind _returnvalue_5 (UserInterface|CreateWidget "/Game/UserInterface/Notification_HUD.Notification_HUD_C" 0 "Settlement is now a city"))
        (UserInterface|Viewport|AddtoViewport _returnvalue_5 0)
        (else
          (bind _returnvalue_6 (UserInterface|CreateWidget "/Game/UserInterface/Notification_HUD.Notification_HUD_C" 0 "          Could not upgrade  
(2 wheat and 3 ore required)"))
          (UserInterface|Viewport|AddtoViewport _returnvalue_6 0)))
      (else
        (bind _returnvalue_7 (Class|Settlement|StealResource "PLAYER1"))
        (if _returnvalue_7
          (bind _returnvalue_8 (UserInterface|CreateWidget "/Game/UserInterface/Notification_HUD.Notification_HUD_C" 0 "Resource stolen"))
          (UserInterface|Viewport|AddtoViewport _returnvalue_8 0)
          (else
            (bind _returnvalue_9 (Class|Settlement|BoughtChecker))
            (if (not _returnvalue_9)
              (bind _returnvalue_10 (Class|Settlement|SettlementBuyer "PLAYER1"))
              (if _returnvalue_10
                (bind _returnvalue_11 (UserInterface|CreateWidget "/Game/UserInterface/Notification_HUD.Notification_HUD_C" 0 "Settlement bought"))
                (UserInterface|Viewport|AddtoViewport _returnvalue_11 0)
                (else
                  (bind _returnvalue_12 (UserInterface|CreateWidget "/Game/UserInterface/Notification_HUD.Notification_HUD_C" 0 "                  Could not buy settlement 
(1 wood, 1 grain, 1 brick and 1 lumber required)"))
                  (UserInterface|Viewport|AddtoViewport _returnvalue_12 0))))))))
    (else
      (bind _returnvalue_13 (UserInterface|CreateWidget "/Game/UserInterface/Notification_HUD.Notification_HUD_C" 0 "Not your turn"))
      (UserInterface|Viewport|AddtoViewport _returnvalue_13 0))))

(fn ConstructionScript)