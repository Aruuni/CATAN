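; Player camera pawn for a Catan game that orbits, zooms and glides to focus on clicked actors.
; A short delay on click separates a hold, which enables axis-driven rotation, from a tap, which traces under the cursor and lerps to the hit actor via timeline.
; Zoom adjusts a clamped spring arm length, and Tick clamps pitch.
; BeginPlay also creates the HUD, adds the input mapping context and finds the GameManager.
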(event Custom|MoveTo%20Focus%20ACTOR
  (params (Focus%20Actor :type Actor%20Object%20Reference))
  ;[1 1 1] Actor focus functionality
  (bind _animcurve (Timeline|FocusTimeline PlayFromStart)
    (:Update
      (Transformation|SetActorLocation (Math|Vector|Lerp(Vector) (Transformation|GetActorLocation) (Transformation|GetActorLocation Focus%20Actor) _animcurve) false false))))

(event EventBeginPlay
  ;[1 1 1] "Constructor"
  (bind _returnvalue (UserInterface|CreateWidget "/Game/UserInterface/Catan_HUD.Catan_HUD_C"))
  (bind _output_get (Variables|Default|SetMenu _returnvalue))
  (UserInterface|Viewport|AddtoViewport _output_get 0)
  (bind _asplayer_controller (Utilities|Casting|CastToPlayerController (Pawn|GetController)))
  (Utilities|IsValid _asplayer_controller
    (:Is%20Valid
      (Input|AddMappingContext (PlayerController|LocalPlayerSubsystems|GetEnhancedInputLocalPlayerSubsystem _asplayer_controller) "/Game/Blueprints/GameMode/Inputs/Inputs.Inputs" 0 "(bIgnoreAllPressedKeysUntilRelease=True,bForceImmediately=False)")
      (bind _returnvalue_2 (Actor|GetActorOfClass "/Script/The_Settlers.GameManager"))
      (Variables|Default|SetGameManager _returnvalue_2))))

(event EventTick
  (params (DeltaSeconds :type Float%20%28single-precision%29))
  ;[1 1 1] Camera Angle clamp
  (CallFunction|CameraClamp))

(event Input|ActionEvents|InputActionCLICK
  (params (Key :type Key%20Structure :default "None"))
  ;[1 1 1] Mouse right click handling
  (:Pressed
    (Utilities|FlowControl|Delay 0.1)
    (CallFunction|HandleMouseClick Key))
  (:Released
    (Variables|Default|SetClickHeld false)))

(event Input|ActionEvents|InputActionZOOM_IN
  (params (Key :type Key%20Structure :default "None"))
  ;[1 1 1] Zoom functionality
  (:Pressed
    (CallFunction|ZOOM -1e+02)))

(event Input|ActionEvents|InputActionZOOM_OUT
  (params (Key :type Key%20Structure :default "None"))
  ;[1 1 1] Zoom functionality
  (:Pressed
    (CallFunction|ZOOM 1e+02)))

(event Input|AxisEvents|InputAxisROTATE_HOZ
  (params (AxisValue :type Float%20%28single-precision%29))
  ;[1 1 1] Rotation clamping
  (if (Variables|Default|GetClickHeld)
    (Class|Actor|AddActorWorldRotation (Math|Rotator|MakeRotator 0.0 0.0 (* AxisValue (Variables|Default|GetRotation%20speed))))))

(event Input|AxisEvents|InputAxisROTATE_VER
  (params (AxisValue :type Float%20%28single-precision%29))
  ;[1 1 1] Rotation clamping
  (if (Variables|Default|GetClickHeld)
    (Transformation|AddActorLocalRotation (Math|Rotator|MakeRotator 0.0 (* AxisValue (Variables|Default|GetRotation%20speed)) 0.0) false false)))

(fn ConstructionScript
  (Variables|Default|SetTarget%20Arm%20Length (Variables|/Script/Engine.SpringArmComponent|GetTargetArmLength (Variables|Default|GetSpringArm))))

(fn CheckifClickHitActor
  (bind _returnvalue (Game|GetPlayerController 0))
  (bind _hitresult (Game|Player|GetHitResultUnderCursorbyChannel _returnvalue "TraceTypeQuery1" true))
  (bind (_bblockinghit _binitialoverlap _time _distance _location _impactpoint _normal _impactnormal _physmat _hitactor) (Collision|BreakHitResult _hitresult))
  (return _bblockinghit _hitactor))

(fn HandleMouseClick
  (params (Key :type Key%20Structure :default "None"))
  (bind _returnvalue (Game|GetPlayerController 0))
  (bind (_bblockinghit _hitactor) (CallFunction|CheckifClickHitActor))
  (bind _returnvalue_2 (Game|Player|IsInputKeyDown _returnvalue Key))
  (if _returnvalue_2
    (Variables|Default|SetClickHeld _returnvalue_2)
    (elif _bblockinghit
      (bind _output_get (Variables|Default|SetHit%20Actor _hitactor))
      (CallFunction|MovetoFocusACTOR _output_get))))

(fn ZOOM
  (params (Zoom%20Speed :type Float%20%28double-precision%29))
  (Variables|/Script/Engine.SpringArmComponent|SetTargetArmLength (Variables|Default|GetSpringArm) (Math|Float|Clamp(Float) (+ Zoom%20Speed (Variables|/Script/Engine.SpringArmComponent|GetTargetArmLength (Variables|Default|GetSpringArm))) (Variables|Default|GetZoomMin) (Variables|Default|GetZoomMax))))

(fn CameraClamp
  (bind _returnvalue (Transformation|GetActorRotation))
  (bind _y_limit_min (Variables|Default|GetY-Limit%20min))
  (bind _y_limit_max (Variables|Default|GetY-Limit%20Max))
  (bind _returnvalue_2 (< (.pitch _returnvalue) _y_limit_min))
  (if (or _returnvalue_2 (> (.pitch _returnvalue) _y_limit_max))
    (Transformation|SetActorRotation (Math|Rotator|MakeRotator 0.0 (Math|Float|SelectFloat _y_limit_min _y_limit_max _returnvalue_2) (.yaw _returnvalue)))))